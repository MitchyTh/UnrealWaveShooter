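; VoiceBlast is an ability actor that damages Basic_Enemy pawns it touches.
; Each Tick it runs a small sphere overlap at its location for Pawns, ignoring player 0's character.
; Every pawn found adds score on BP_ThirdPersonCharacter before the enemy cast; an enemy then takes fixed damage and the blast calls DestroyActor.
; Detection relies on this polling, as ActorBeginOverlap is empty.
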(event `self.ReceiveTick`
  (params (DeltaSeconds :type "Float (single-precision)"))
  (bind _outactors (`KismetSystemLibrary.SphereOverlapActors` (`self.K2_GetActorLocation`) 55.0 (`|MakeArray` "ObjectTypeQuery3" :!type "EObjectTypeQuery Enum") null (`|MakeArray` (`GameplayStatics.GetPlayerCharacter` 0) :!type "Actor Object Reference")))
  (bind _asbp_third_person_character (cast `/Game/ThirdPerson/Blueprints/BP_ThirdPersonCharacter` (`GameplayStatics.GetPlayerCharacter` 0)))
  (for _array_element _outactors
    (`/Game/ThirdPerson/Blueprints/BP_ThirdPersonCharacter.AddScore` _asbp_third_person_character)
    (bind _asbasic_enemy (cast `/Game/Blueprints/Enemies/Basic_Enemy` _array_element))
    (`/Game/Blueprints/Enemies/Basic_Enemy.TakeDamage` _asbasic_enemy 20.0)
    (`self.K2_DestroyActor`)))

(fn `UserConstructionScript`)