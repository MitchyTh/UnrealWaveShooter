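; Basic enemy character that takes damage, flashes red when hit and reports its death to the game mode.
; BeginPlay applies a dynamic material instance to the mesh, which TakeDamage tints red briefly before resetting to white.
; The same event subtracts Health and, at zero or below, destroys the actor and calls EnemyDies on BP_ThirdPersonGameMode.
; UpdateSpeedWalk sets the movement component's max walk speed.
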(event `self.ReceiveBeginPlay`
  (bind _returnvalue (`KismetMaterialLibrary.CreateDynamicMaterialInstance` "/Game/Materials/Hit_Material.Hit_Material" "DynamicMaterial"))
  (bind _output_get (set `self.DynamicMaterial` _returnvalue))
  (`PrimitiveComponent.SetMaterial` (`self.Mesh`) 0 _output_get))

(event `TakeDamage`
  (params (Amount :type "Float (double-precision)"))
  (`|ExecutionSequence`
    (:`then_0`
      (`MaterialInstanceDynamic.SetVectorParameterValue` (`self.DynamicMaterial`) "BaseColor" (struct :`R` 1.0 :`B` 0.047706 :`A` 1.0))
      (`KismetSystemLibrary.Delay` 0.2)
      (`MaterialInstanceDynamic.SetVectorParameterValue` (`self.DynamicMaterial`) "BaseColor" (struct :`R` 1.0 :`G` 1.0 :`B` 1.0 :`A` 1.0)))
    (:`then_1`
      (bind _output_get (set `self.Health` (- (`self.Health`) Amount)))
      (if (<= _output_get 0.0)
        (`self.K2_DestroyActor`)
        (bind _asbp_third_person_game_mode (cast `/Game/ThirdPerson/Blueprints/BP_ThirdPersonGameMode` (`GameplayStatics.GetGameMode`)))
        (`/Game/ThirdPerson/Blueprints/BP_ThirdPersonGameMode.EnemyDies` _asbp_third_person_game_mode)))))

(fn `UpdateSpeedWalk`
  (params (WalkSpeed :type "Float (double-precision)"))
  (set `CharacterMovementComponent.MaxWalkSpeed` WalkSpeed (`self.CharacterMovement`)))

(fn `UserConstructionScript`)