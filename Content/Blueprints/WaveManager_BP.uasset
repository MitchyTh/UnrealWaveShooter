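; Wave manager that runs endless, escalating rounds of enemy spawns.
; On BeginPlay it caches all SpawnPoint actors and starts the first wave.
; Each wave sizes its enemy count linearly from the round number and calls SpawnEnemy on randomly picked spawn points in one loop, without delay.
; The EnemyDies event decrements the remaining count and immediately starts the next wave when it reaches zero.
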(event `self.ReceiveBeginPlay`
  (bind _outactors (`GameplayStatics.GetAllActorsOfClass` "/Game/Blueprints/Spawner/SpawnPoint.SpawnPoint_C"))
  (set `self.Spawners` _outactors)
  (set `self.RoundNumber` 0)
  (`self.StartNextWave`))

(event `StartNextWave`
  (bind _returnvalue (* (`self.RoundNumber`) 5))
  (set `self.RoundNumber` (+ (`self.RoundNumber`) 1))
  (set `self.EnemiesToSpawn` _returnvalue)
  (set `self.EnemiesRemaining` _returnvalue)
  (for _ (range (+ (`self.EnemiesToSpawn`) 1))
    (`/Game/Blueprints/Spawner/SpawnPoint.SpawnEnemy` (`KismetArrayLibrary.Array_Random` (`self.Spawners`)))
    (set `self.EnemiesToSpawn` (- (`self.EnemiesToSpawn`) 1))))

(event `EnemyDies`
  (set `self.EnemiesRemaining` (- (`self.EnemiesRemaining`) 1))
  (if (== (`self.EnemiesRemaining`) 0)
    (`self.StartNextWave`)))

(fn `UserConstructionScript`)